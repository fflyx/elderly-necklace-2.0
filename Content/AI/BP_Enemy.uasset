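; BP_Enemy is an AI enemy that chases the player and deals contact damage.
; On BeginPlay it calls Roaming, a simple move with no goal location set, then after a short delay issues a move toward the player character.
; Hurtbox hits damage whatever actor they touch, without filtering, and a DoOnce reset after HitDelay throttles repeat hits.
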(event OnComponentHit(Hurtbox)
  (params (HitComponent :type Primitive%20Component%20Object%20Reference) (OtherActor :type Actor%20Object%20Reference) (OtherComp :type Primitive%20Component%20Object%20Reference) (NormalImpulse :type Vector :default "0, 0, 0") (Hit :type Hit%20Result%20Structure%20%28by%20ref%29))
  (bind _self self)
  (Utilities|FlowControl|DoOnce false :!label _label
    (:Completed
      (Game|Damage|ApplyDamage OtherActor 1e+01 (AI|GetAIController _self) _self)
      (Utilities|FlowControl|Delay (Variables|Default|GetHitDelay))
      (goto _label Reset))))

(event EventBeginPlay
  (CallFunction|Roaming)
  (Utilities|FlowControl|Delay 3.0)
  (CallFunction|BeginChase))

(fn ConstructionScript)

(fn BeginChase
  (AI|Navigation|SimpleMovetoActor (AI|GetAIController self) (Game|GetPlayerCharacter 0))
  (return))

(fn Roaming
  (AI|Navigation|SimpleMovetoLocation (AI|GetAIController self) (Math|Vector|MakeVector 0.0 0.0 0.0))
  (return))