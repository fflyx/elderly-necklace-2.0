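; BP_MPC is a player controller that opens the main menu when play begins.
; BeginPlay adds the default Enhanced Input mapping context, shows the menu, switches to UI-only input focused on it and enables the mouse cursor, all only if the input subsystem is valid.
; UI_ShowMainMenu creates the WBP_MainMenu widget once, caches it, adds it to the viewport and returns it.
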(event EventBeginPlay
  (bind _returnvalue (PlayerController|LocalPlayerSubsystems|GetEnhancedInputLocalPlayerSubsystem))
  (Utilities|IsValid _returnvalue
    (:Is%20Valid
      (Input|AddMappingContext _returnvalue "/Game/Input/IMC_Default.IMC_Default" 0 "(bIgnoreAllPressedKeysUntilRelease=True,bForceImmediately=False,bNotifyUserSettings=False)")
      (bind _wbp_mainmenu (CallFunction|UIShowMainMenu))
      (Input|SetInputModeUIOnly self _wbp_mainmenu "DoNotLock" false)
      (Variables|Default|SetbShowMouseCursor true))))

(fn ConstructionScript)

(fn UIShowMainMenu
  (Utilities|IsValid (Variables|Default|GetWBP_MainMenu)
    (:Is%20Valid
      _)
    (:Is%20Not%20Valid
      (bind _returnvalue (UserInterface|CreateWidget "/Game/Widgets/WBP_MainMenu.WBP_MainMenu_C" self))
      (Variables|Default|SetWBP_MainMenu _returnvalue)))
  (UserInterface|Viewport|AddtoViewport (Variables|Default|GetWBP_MainMenu) 0)
  (return (Variables|Default|GetWBP_MainMenu)))